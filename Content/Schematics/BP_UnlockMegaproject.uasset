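; Schematic unlock that unlocks megaprojects of a configured class when applied.
; On apply, it calls the parent, then, with authority only, unlocks every existing megaproject whose class is a child of that class.
; For UI, it supplies its own name, description and icons through an info-only reward widget and borrows stinger data from BP_UnlockInfoOnly's class default object.
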(event `self.OnApply`
  (params (unlockSubsystem :type "FGUnlockSubsystem Object Reference"))
  (bind _returnvalue (`AVRPMegaprojectsManager.Get` unlockSubsystem))
  (`parent.OnApply` unlockSubsystem)
  (bind _returnvalue_2 (`AVRPMegaprojectsManager.GetMegaprojects` _returnvalue))
  (if (`Actor.HasAuthority` _returnvalue)
    (for _array_element _returnvalue_2
      (if (`KismetMathLibrary.ClassIsChildOf` (`GameplayStatics.GetObjectClass` _array_element) (`self.megaproject`))
        (`AVRPMegaprojectSubsystemBase.UnlockMegaproject` _array_element)))))

(fn `GetCost`
  (params (UnlockStructIndex :type Integer))
  (returns (cost :type "Array of ItemAmount Structure"))
  (return))

(fn `GetStingerWidgetRewardData`
  (returns (StingerRewardTypes :type "Set of FGStingerWidgetRewardData Class Reference"))
  (bind _stingerrewardtypes (`/Game/FactoryGame/Unlocks/BP_UnlockInfoOnly.GetStingerWidgetRewardData` (`BlueprintReflectionLibrary.GetClassDefaultObject` "/Game/FactoryGame/Unlocks/BP_UnlockInfoOnly.BP_UnlockInfoOnly_C")))
  (return _stingerrewardtypes))

(fn `GetUnlockDataStruct`
  (returns (UnlockDataStruct :type "Array of /Game/FactoryGame/Unlocks/FUnlockDataStruct Structure"))
  (return (`|MakeArray` (make `/Game/FactoryGame/Unlocks/FUnlockDataStruct` (`self.mUnlockName`) (`self.mUnlockDescription`) (`self.mUnlockIconSmall`) (`self.mUnlockIconBig`) 0 0 self))))

(fn `GetUnlockRewardWidgets`
  (params (OwningPlayer :type "PlayerController Object Reference") (SchematicClass :type "FGSchematic Class Reference") (TradingPostWidget :type "UserWidget Object Reference"))
  (returns (Widgets :type "Array of UserWidget Object Reference"))
  (bind _returnvalue (`|CreateWidget` "/Game/FactoryGame/Buildable/Factory/TradingPost/Widget_RewardInfoOnly.Widget_RewardInfoOnly_C" OwningPlayer (`self.mUnlockIconBig`) (`self.mUnlockIconCategory`) SchematicClass TradingPostWidget (`self.mUnlockName`) (`self.mUnlockDescription`)))
  (return (`|MakeArray` _returnvalue :!type "UserWidget Object Reference")))